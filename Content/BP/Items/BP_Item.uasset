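; BP_Item is an item actor that shows an interaction prompt while a player is in range.
; Its in-range event creates an Interaccion_Widget for that player and attaches it in a runtime-added screen-space widget component, if none exists.
; The out-of-range event destroys that component.
; Prompt text and attach point come from separate getter functions, defaulting to "Interact" and the root component.
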(event `/Game/Elementos_Interacciones/Interacciones.DentrodelRango`
  (params (Player :type "/Game/BP/BP_PJ Object Reference"))
  (`self.InteraccionWidget`
    (:`then`)
    (:`else`
      (bind _returnvalue (`|CreateWidget` "/Game/Elementos_Interacciones/Interaccion_Widget.Interaccion_Widget_C" (cast `PlayerController` (`Pawn.GetController` Player) :!pure true) (`self.ObtenerTextoInteraccion`)))
      (bind _returnvalue_2 (`AddComponent|NODE_AddWidgetComponent-0`))
      (bind _output_get (set `self.InteraccionWidget` _returnvalue_2))
      (`WidgetComponent.SetWidget` _output_get _returnvalue)
      (`WidgetComponent.SetWidgetSpace` _output_get "Screen")
      (`WidgetComponent.SetDrawAtDesiredSize` _output_get true)
      (`PrimitiveComponent.SetCollisionEnabled` _output_get "NoCollision")
      (`SceneComponent.K2_AttachToComponent` _output_get (`self.ObtenerTextoAttach`) "None" "SnapToTarget" "SnapToTarget" "SnapToTarget" true))))

(event `/Game/Elementos_Interacciones/Interacciones.FueradeRango`
  (bind _interaccionwidget (`self.InteraccionWidget`)
    (:`then`
      (`ActorComponent.K2_DestroyComponent` _interaccionwidget))
    (:`else`)))

(fn `ObtenerTextoAttach`
  (returns (Componente :type "SceneComponent Object Reference"))
  (return (`self.DefaultSceneRoot`)))

(fn `ObtenerTextoInteraccion`
  (returns (Texto :type Text))
  (return "Interact"))

(fn `UserConstructionScript`)