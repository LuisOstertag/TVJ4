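; BP_Armas is a weapon actor that players pick up through interaction, carry, drop and fire.
; EstadodelArma toggles Drop (physics mesh, overlap sphere) and Equipada (no physics or collision, mesh transform reset); it starts dropped.
; Interaction passes the weapon to the player's AgarrarArma and equips it.
; Disparo spawns two actors at the muzzle socket, aiming the bullet velocity at a far point along the camera's forward vector.
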(event `self.ReceiveBeginPlay`
  (`self.EstadodelArma` "NewEnumerator0"))

(event `/Game/Elementos_Interacciones/Interacciones.EnInteraccion`
  (params (Player :type "/Game/BP/BP_PJ Object Reference"))
  (`/Game/BP/BP_PJ.AgarrarArma` Player self)
  (`self.EstadodelArma` "NewEnumerator1"))

(fn `Disparo`
  (params (PlayerCamera :type "CameraComponent Object Reference"))
  (bind _returnvalue (`SceneComponent.GetSocketLocation` (`self.SkeletalMesh`) "SOCKET_Muzzle"))
  (`|SpawnActorFromClass` "/Game/BP/Items/BP_Bala.BP_Bala_C" (`KismetMathLibrary.MakeTransform` _returnvalue) "Undefined" "OverrideRootScale" null (* (`KismetMathLibrary.Normal` (- (+ (`SceneComponent.K2_GetComponentLocation` PlayerCamera) (* (`SceneComponent.GetForwardVector` PlayerCamera) 10000.0)) _returnvalue)) 10000.0) null)
  (`|SpawnActorFromClass` "/Game/BP/Items/BP_MuzzleFlash.BP_MuzzleFlash_C" (`KismetMathLibrary.MakeTransform` _returnvalue) "Undefined" "OverrideRootScale" null null))

(fn `Drop`
  (`self.EstadodelArma` "NewEnumerator0"))

(fn `EstadodelArma`
  (params (EstadodelArma :type "/Game/BP/Items/Armas/EstadodelArma Enum" :default "NewEnumerator0"))
  (bind _skeletalmesh (`self.SkeletalMesh`))
  (bind _skeletalmesh_2 (`self.SkeletalMesh`))
  (bind _output_get (set `self.Estadodel Arma` EstadodelArma))
  (switch `/Game/BP/Items/Armas/EstadodelArma` _output_get
    (:`NewEnumerator0`
      (`PrimitiveComponent.SetCollisionProfileName` (`self.Sphere`) "OverlapAllDynamic" true)
      (`PrimitiveComponent.SetSimulatePhysics` _skeletalmesh_2 true)
      (`PrimitiveComponent.SetCollisionProfileName` _skeletalmesh_2 "DroppedGun" true))
    (:`NewEnumerator1`
      (`PrimitiveComponent.SetCollisionProfileName` (`self.Sphere`) "NoCollision" true)
      (`PrimitiveComponent.SetSimulatePhysics` _skeletalmesh false)
      (`PrimitiveComponent.SetCollisionProfileName` _skeletalmesh "NoCollision" true)
      (`SceneComponent.ResetRelativeTransform` _skeletalmesh))))

(fn `ObtenerTextoAttach`
  (returns (Componente :type "SceneComponent Object Reference"))
  (return (`self.SkeletalMesh`)))

(fn `ObtenerTextoInteraccion`
  (returns (Texto :type Text))
  (return "Pick Up"))

(fn `UserConstructionScript`
  (`parent.UserConstructionScript`))