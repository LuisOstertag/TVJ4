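; BP_EnemigoNormal2 is a zombie enemy that melee-attacks the player, BP_PJ.
; Box overlap plays the attack montage, using Atacando to block re-triggering until it completes.
; Brazo_Ataque overlap subtracts DañoAPersonaje from the player's Vida through a DoOnce that resets after a short delay and debug print.
; A separate Ataque function also plays a montage, but its damage step is disconnected.
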(event `self.Brazo_Ataque.OnComponentBeginOverlap`
  (params (OverlappedComponent :type "PrimitiveComponent Object Reference") (OtherActor :type "Actor Object Reference") (OtherComp :type "PrimitiveComponent Object Reference") (OtherBodyIndex :type Integer) (bFromSweep :type Boolean) (SweepResult :type "HitResult Structure (by ref)"))
  ;[1 1 1] Enemigo baja vida y aplica fuerza al PJ
  (bind _asbp_pj (cast `/Game/BP/BP_PJ` OtherActor))
  (`/Engine/EditorBlueprintResources/StandardMacros.DoOnce` false :!label _label
    (:`Completed`
      (bind _output_get (set `/Game/BP/BP_PJ.Vida` (- (`/Game/BP/BP_PJ.Vida` _asbp_pj) (`self.DañoAPersonaje`)) _asbp_pj))
      (`KismetSystemLibrary.Delay` 0.5)
      (`KismetSystemLibrary.PrintString` (`KismetStringLibrary.Conv_DoubleToString` _output_get))
      (goto _label :!via `Reset`))))

(event `self.Box.OnComponentBeginOverlap`
  (params (OverlappedComponent :type "PrimitiveComponent Object Reference") (OtherActor :type "Actor Object Reference") (OtherComp :type "PrimitiveComponent Object Reference") (OtherBodyIndex :type Integer) (bFromSweep :type Boolean) (SweepResult :type "HitResult Structure (by ref)"))
  ;[1 1 1] Enemigo pega y reproduce anim.
  (cast `/Game/BP/BP_PJ` OtherActor)
  (if (not (`self.Atacando`))
    (set `self.Atacando` true)
    (`|PlayMontage` (`self.Mesh`) "/Game/Modelos/PlaceHolder/Animaciones/Zombie_Attack_Montage.Zombie_Attack_Montage"
      (:`OnCompleted`
        (set `self.Atacando` false)))))

(fn `Ataque`
  (params (Cantidad :type "Float (double-precision)"))
  (set `self.Atacando` true)
  (`self.PlayAnimMontage` (`self.Zombie_Ataque_Montaje`))
  (set `self.Atacando` false)
  (`KismetSystemLibrary.PrintString` (`KismetStringLibrary.Conv_DoubleToString` 0.0)))

(fn `UserConstructionScript`)