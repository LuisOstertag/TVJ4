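; Shooting target actor for the LPSP sample that reacts to point and radial damage.
; Point damage on an active target plays the knockdown animation and sound, deactivates it, then raises and reactivates it after a random delay.
; Radial damage skips the active check, spawns a destroyed-target actor at the mesh transform and removes the target permanently.
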(event `/Game/LPSPSample/Core/BPI_LPSP_Damageable.On Receive Damage Point`
  ;[1 0.03719 0] Point Damage
  (if (`self.Active`)
    (`GameplayStatics.SpawnSoundAtLocation` "/Game/LPSPSample/Audio/SC_Target_Down.SC_Target_Down" (`SceneComponent.K2_GetComponentLocation` (`self.Mesh`)) (struct) 1.0 1.0 0.0 null null)
    (`SkeletalMeshComponent.PlayAnimation` (`self.Mesh`) "/Game/LPSPSample/Art/Environment/Damageables/A_Target_Down.A_Target_Down" false)
    (set `self.Active` false)
    (`KismetSystemLibrary.Delay` (`KismetMathLibrary.RandomFloatInRange` 1.0 10.0))
    (set `self.Active` true)
    (`SkeletalMeshComponent.PlayAnimation` (`self.Mesh`) "/Game/LPSPSample/Art/Environment/Damageables/A_Target_Up.A_Target_Up" false)
    (`GameplayStatics.SpawnSoundAtLocation` "/Game/LPSPSample/Audio/SC_Target_Up.SC_Target_Up" (`SceneComponent.K2_GetComponentLocation` (`self.Mesh`)) (struct) 1.0 1.0 0.0 null null)))

(event `/Game/LPSPSample/Core/BPI_LPSP_Damageable.On Receive Damage Radial`
  ;[1 0.1603 0] Radial Damage
  (`|SpawnActorFromClass` "/Game/LPSPSample/Useable/Damageables/BP_LPSP_Destroyed_Target.BP_LPSP_Destroyed_Target_C" (`SceneComponent.K2_GetComponentToWorld` (`self.Mesh`)) "AlwaysSpawn" "OverrideRootScale" null null)
  (`self.K2_DestroyActor`))

(fn `UserConstructionScript`)